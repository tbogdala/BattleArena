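; BP_PlayerHUD is the player HUD that shows a crosshair and the owning player's win and loss counts.
; BeginPlay creates the stats widget and adds it to the viewport.
; DrawHUD draws the crosshair near screen center, offset horizontally by twice as much as vertically.
; It then refreshes the widget's text every draw from BattleArenaPlayerState, rather than on score changes.
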(event EventBeginPlay
  (bind _returnvalue (UserInterface|CreateWidget "/Game/PlayerBlueprints/Widget_Stats.Widget_Stats_C"))
  (bind _output_get (Variables|Default|SetStatsWidget _returnvalue))
  (UserInterface|Viewport|AddtoViewport _output_get 0))

(event EventDrawHUD
  (params (SizeX :type Integer) (SizeY :type Integer))
  (bind _crosshairhalfsize (Variables|Default|GetCrosshairHalfSize))
  (Canvas|DrawTexture "/Game/PlayerBlueprints/Crosshair.Crosshair" (Math|Conversions|ToFloat(Integer) (- (/ SizeX 2) (* _crosshairhalfsize 2))) (Math|Conversions|ToFloat(Integer) (- (/ SizeY 2) _crosshairhalfsize)) 2e+01 2e+01 0.0 0.0 1.0 1.0 "(R=1.000000,G=1.000000,B=1.000000,A=1.000000)")
  (bind _asbattle_arena_player_state (Utilities|Casting|CastToBattleArenaPlayerState (Variables|/Script/Engine.Controller|GetPlayerState (Variables|Default|GetPlayerOwner))))
  (Rendering|Components|TextRender|SetText (Variables|/Game/PlayerBlueprints/Widget_Stats.Widget_Stats_C|GetTextBlock_Wins (Variables|Default|GetStatsWidget)) (Utilities|Text|ToText(Integer) (Variables|/Script/BattleArena.BattleArenaPlayerState|GetWins _asbattle_arena_player_state)))
  (Rendering|Components|TextRender|SetText (Variables|/Game/PlayerBlueprints/Widget_Stats.Widget_Stats_C|GetTextBlock_Losses (Variables|Default|GetStatsWidget)) (Utilities|Text|ToText(Integer) (Variables|/Script/BattleArena.BattleArenaPlayerState|GetLosses _asbattle_arena_player_state))))

(fn ConstructionScript)