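; BP_GrappleProjectile is a projectile that explodes with a radial force on hit, despite its grapple name.
; On Hit it spawns a BP_GrenadeRadialForce at the impact point, activates its high-strength force, plays an explosion sound and destroys itself.
; Cleanup of the force actor sits behind a short Delay after the projectile's own DestroyActor, so it may never run.
; A BeginPlay timer destroys projectiles after five seconds.
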(event EventBeginPlay
  ;[1 1 1] 5 second ttl
  (Utilities|FlowControl|Delay 5.0)
  (Actor|DestroyActor))

(event Collision|EventHit
  (params (MyComp :type Primitive%20Component%20Object%20Reference) (Other :type Actor%20Object%20Reference) (OtherComp :type Primitive%20Component%20Object%20Reference) (bSelfMoved :type Boolean) (HitLocation :type Vector :default "0, 0, 0") (HitNormal :type Vector :default "0, 0, 0") (NormalImpulse :type Vector :default "0, 0, 0") (Hit :type Hit%20Result%20Structure%20%28by%20ref%29))
  (bind _returnvalue (Game|SpawnActorfromClass "/Game/PlayerBlueprints/BP_GrenadeRadialForce.BP_GrenadeRadialForce_C" (Math|Conversions|ToTransform(Vector) HitLocation) "AdjustIfPossibleButAlwaysSpawn" (Components|GetOwner MyComp) 0))
  (Variables|/Script/Engine.RadialForceComponent|SetForceStrength (Variables|/Script/Engine.RadialForceActor|GetForceComponent _returnvalue) 1e+06)
  (Components|Activation|Activate (Variables|/Script/Engine.RadialForceActor|GetForceComponent _returnvalue) false)
  (Utilities|FlowControl|Sequence
    (:then_0
      (Audio|PlaySoundatLocation "/Game/Sounds/Explosion_Cue.Explosion_Cue" HitLocation "0, 0, 0" 1.0 1.0 0.0 0 0 0))
    (:then_1
      (Actor|DestroyActor)
      (Utilities|FlowControl|Delay 0.5)
      (Actor|DestroyActor _returnvalue))))

(fn ConstructionScript)