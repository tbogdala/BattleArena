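; BP_Killbox is a killbox actor that tells the game mode when battle characters hit it.
; On BeginPlay it registers itself with BP_BaseGameMode through SetKillBox.
; Its Hit event calls ActorHitKillBox on the game mode, passing BP_BattleCharacter hits along but supplying no actor for AI_BattleCharacter hits.
; Both events run only with authority, leaving the response to the game mode.
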(event EventBeginPlay
  ;[1 1 1] register the killbox with the game mode
  (Networking|SwitchHasAuthority
    (:Authority
      (bind _asbp_base_game_mode (Utilities|Casting|CastToBP_BaseGameMode (Game|GetGameMode)))
      (Class|BattleArenaGameModeBase|SetKillBox _asbp_base_game_mode self))))

(event Collision|EventHit
  (params (MyComp :type Primitive%20Component%20Object%20Reference) (Other :type Actor%20Object%20Reference) (OtherComp :type Primitive%20Component%20Object%20Reference) (bSelfMoved :type Boolean) (HitLocation :type Vector :default "0, 0, 0") (HitNormal :type Vector :default "0, 0, 0") (NormalImpulse :type Vector :default "0, 0, 0") (Hit :type Hit%20Result%20Structure%20%28by%20ref%29))
  ;[1 1 1] tell the game that a player hit the killbox
  (Networking|SwitchHasAuthority
    (:Authority
      (bind _asbp_battle_character (Utilities|Casting|CastToBP_BattleCharacter Other)
        (:then
          (bind _asbp_base_game_mode (Utilities|Casting|CastToBP_BaseGameMode (Game|GetGameMode)))
          (Class|BattleArenaGameModeBase|ActorHitKillBox _asbp_base_game_mode _asbp_battle_character))
        (:CastFailed
          (Utilities|Casting|CastToAI_BattleCharacter Other)
          (bind _asbp_base_game_mode_2 (Utilities|Casting|CastToBP_BaseGameMode (Game|GetGameMode)))
          (Class|BattleArenaGameModeBase|ActorHitKillBox _asbp_base_game_mode_2))))))

(fn ConstructionScript)